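; Player character with movement, sprinting, item pickup and ore mining.
; BP_GameModeBase_01 handles inventory and pause requests, and its ConfigueUI state gates movement, look and sprint to game mode.
; Capsule overlaps add BPI_PickUp items to BPInventory and create a hidden inventory widget if missing.
; Interact sphere-traces forward, calls GetHit on Ruby, Cuivre or Fer ores and plays a pickaxe sound, with persistent debug drawing left on.
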(event OnComponentBeginOverlap(CapsuleComponent)
  (params (OverlappedComponent :type Primitive%20Component%20Object%20Reference) (OtherActor :type Actor%20Object%20Reference) (OtherComp :type Primitive%20Component%20Object%20Reference) (OtherBodyIndex :type Integer) (bFromSweep :type Boolean) (SweepResult :type Hit%20Result%20Structure%20%28by%20ref%29))
  ;[1 1 1] PickObject
  (Variables|Default|SetDetectMinerai true)
  (Variables|Default|GetInventoryWidget
    (:then
      _)
    (:else
      (bind _returnvalue (UserInterface|CreateWidget "/Game/InterfaceUtilisateur/Widget/WB_InventairePlayerUI.WB_InventairePlayerUI_C"))
      (bind _output_get (Variables|Default|SetInventoryWidget _returnvalue))
      (UserInterface|Viewport|AddtoViewport _output_get 0)
      (Widget|SetVisibility (Variables|Default|GetInventoryWidget) "Hidden")))
  (for _array_element (Collision|GetOverlappingActors "/Game/Blueprints/Inventory/BP_Item.BP_Item_C" :!class /Script/Engine.Actor)
    (if (Utilities|DoesObjectImplementInterface _array_element "/Game/Blueprints/Inventory/BPI_PickUp.BPI_PickUp_C")
      (bind _item (Class|BPIPickUp|PickUpItem(Message) _array_element))
      (Default|AddItemtoInventory (Variables|Default|GetBP_Inventory) _item)
      (Variables|Default|GetInventoryWidget
        (:then)
        (:else
          (bind _returnvalue_2 (UserInterface|CreateWidget "/Game/InterfaceUtilisateur/Widget/WB_InventairePlayerUI.WB_InventairePlayerUI_C"))
          (bind _output_get_2 (Variables|Default|SetInventoryWidget _returnvalue_2))
          (UserInterface|Viewport|AddtoViewport _output_get_2 0)
          (Widget|SetVisibility (Variables|Default|GetInventoryWidget) "Hidden"))))))

(event EventBeginPlay
  (bind _returnvalue (Actor|GetActorOfClass "/Game/Blueprints/Characters/BP_GameModeBase_01.BP_GameModeBase_01_C"))
  (Variables|Default|SetBP%20Game%20Mode%2001%20Ref _returnvalue))

(event Input|ActionEvents|InputActionSprint
  (params (Key :type Key%20Structure :default "None"))
  (bind _charactermovement (Variables|Character|GetCharacterMovement))
  (bind _bp_game_mode_01_ref (Variables|Default|GetBP%20Game%20Mode%2001%20Ref))
  (bind _configueui (Variables|/Game/Blueprints/Characters/BP_GameModeBase_01.BP_GameModeBase_01_C|GetConfigueUI _bp_game_mode_01_ref))
  ;[1 1 1] Sprint
  (:Pressed
    (switch Utilities|FlowControl|Switch|SwitchonE_UiList _configueui
      (:NewEnumerator6
        (Variables|/Script/Engine.CharacterMovementComponent|SetMaxWalkSpeed _charactermovement 1.2e+03))))
  (:Released
    (switch Utilities|FlowControl|Switch|SwitchonE_UiList _configueui
      (:NewEnumerator6
        (Variables|/Script/Engine.CharacterMovementComponent|SetMaxWalkSpeed _charactermovement 6e+02)))))

(event Input|ActionEvents|InputActionInventoryPlayer
  (params (Key :type Key%20Structure :default "None"))
  ;[1 1 1] Inventory
  (:Pressed
    (Default|OpenPlayerInventory (Variables|Default|GetBP%20Game%20Mode%2001%20Ref))))

(event Input|ActionEvents|InputActionInteract
  (params (Key :type Key%20Structure :default "None"))
  (bind _returnvalue (Transformation|GetActorLocation))
  (:Pressed
    (bind (_outhit _returnvalue_2) (Collision|SphereTraceForObjects _returnvalue (+ _returnvalue (* (Transformation|GetActorForwardVector) 250)) 5e+01 (Variables|Default|GetObject%20Types) false 0 "Persistent"))
    (if _returnvalue_2
      (Utilities|FlowControl|Sequence
        (:then_0
          (bind _asbp_ruby (Utilities|Casting|CastToBP_Ruby (.HitActor (Collision|BreakHitResult _outhit)))
            (:then
              (Default|GetHit _asbp_ruby))
            (:CastFailed
              (bind _asbp_cuivre (Utilities|Casting|CastToBP_Cuivre (.HitActor (Collision|BreakHitResult _outhit)))
                (:then
                  (Default|GetHit _asbp_cuivre))
                (:CastFailed
                  (bind _asbp_fer (Utilities|Casting|CastToBP_Fer (.HitActor (Collision|BreakHitResult _outhit))))
                  (Default|GetHit _asbp_fer))))))
        (:then_1
          (Audio|PlaySound2D "/Game/Sound/Pioche_1.Pioche_1" 1.0 1.0 0.0 0 0))))))

(event Input|ActionEvents|InputActionPause
  (params (Key :type Key%20Structure :default "None"))
  ;[1 1 1] Pause
  (:Pressed
    (Default|SetPause (Variables|Default|GetBP%20Game%20Mode%2001%20Ref))))

(event Input|AxisEvents|InputAxisMoveForward
  (params (AxisValue :type Float%20%28single-precision%29))
  ;[1 1 1] Movement
  (switch Utilities|FlowControl|Switch|SwitchonE_UiList (Variables|/Game/Blueprints/Characters/BP_GameModeBase_01.BP_GameModeBase_01_C|GetConfigueUI (Variables|Default|GetBP%20Game%20Mode%2001%20Ref))
    (:NewEnumerator6
      (Pawn|Input|AddMovementInput (Transformation|GetActorForwardVector) AxisValue false))))

(event Input|AxisEvents|InputAxisMoveRight
  (params (AxisValue :type Float%20%28single-precision%29))
  ;[1 1 1] Movement
  (switch Utilities|FlowControl|Switch|SwitchonE_UiList (Variables|/Game/Blueprints/Characters/BP_GameModeBase_01.BP_GameModeBase_01_C|GetConfigueUI (Variables|Default|GetBP%20Game%20Mode%2001%20Ref))
    (:NewEnumerator6
      (Pawn|Input|AddMovementInput (Transformation|GetActorRightVector) AxisValue false))))

(event Input|AxisEvents|InputAxisTurnRight
  (params (AxisValue :type Float%20%28single-precision%29))
  ;[1 1 1] Mouse Turn Input
  (switch Utilities|FlowControl|Switch|SwitchonE_UiList (Variables|/Game/Blueprints/Characters/BP_GameModeBase_01.BP_GameModeBase_01_C|GetConfigueUI (Variables|Default|GetBP%20Game%20Mode%2001%20Ref))
    (:NewEnumerator6
      (Pawn|Input|AddControllerYawInput AxisValue))))

(event Input|AxisEvents|InputAxisLookUp/Down
  (params (AxisValue :type Float%20%28single-precision%29))
  ;[1 1 1] Mouse Turn Input
  (switch Utilities|FlowControl|Switch|SwitchonE_UiList (Variables|/Game/Blueprints/Characters/BP_GameModeBase_01.BP_GameModeBase_01_C|GetConfigueUI (Variables|Default|GetBP%20Game%20Mode%2001%20Ref))
    (:NewEnumerator6
      (Pawn|Input|AddControllerPitchInput AxisValue))))

(fn ConstructionScript)

(fn SpendMoney
  (params (Money :type Integer))
  (Variables|Default|SetMoney (- (Variables|Default|GetMoney) Money))
  (return 0))