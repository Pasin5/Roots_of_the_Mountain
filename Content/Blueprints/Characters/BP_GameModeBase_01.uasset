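; Game mode that owns and switches all UI screens: menu, pause, settings, controls, audio, HUD, merchant selection, merchant buy/sell inventories and player inventory.
; On BeginPlay it creates every widget once, stores references and adds all to the viewport, with only the main menu visible.
; GestionUI switches on the ConfigueUI state, showing the matching widget and hiding all others, so screens toggle by visibility rather than being recreated.
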(event Custom|GestionUI
  (switch Utilities|FlowControl|Switch|SwitchonE_UiList (Variables|Default|GetConfigueUI)
    (:NewEnumerator0
      (Widget|SetVisibility (Variables|Default|GetWB%20Menu%20UI%20Ref) "Visible")
      (Widget|SetVisibility (Variables|Default|GetWB%20Pause%20UI%20ref) "Hidden"))
    (:NewEnumerator1
      (Widget|SetVisibility (Variables|Default|GetWB%20Pause%20UI%20ref) "Visible")
      (Widget|SetVisibility (Variables|Default|GetWB%20Settings%20UI%20Ref) "Hidden"))
    (:NewEnumerator2
      (Widget|SetVisibility (Variables|Default|GetWB%20Settings%20UI%20Ref) "Visible")
      (Widget|SetVisibility (Variables|Default|GetWB%20Pause%20UI%20ref) "Hidden"))
    (:NewEnumerator3
      (Widget|SetVisibility (Variables|Default|GetWB%20Controls%20UI%20Ref) "Visible")
      (Widget|SetVisibility (Variables|Default|GetWB%20Pause%20UI%20ref) "Hidden"))
    (:NewEnumerator4
      (Widget|SetVisibility (Variables|Default|GetWB%20Audio%20UI%20Ref) "Visible")
      (Widget|SetVisibility (Variables|Default|GetWB%20Pause%20UI%20ref) "Hidden"))
    (:NewEnumerator5
      (Widget|SetVisibility (Variables|Default|GetWB%20Selection%20Marchand%20UI%20Ref) "Visible")
      (Widget|SetVisibility (Variables|Default|GetWB%20Pause%20UI%20ref) "Hidden"))
    (:NewEnumerator6
      (Widget|SetVisibility (Variables|Default|GetWB%20Game%20UI%20Ref) "Visible")
      (Widget|SetVisibility (Variables|Default|GetWB%20Pause%20UI%20ref) "Hidden"))
    (:NewEnumerator7
      (Widget|SetVisibility (Variables|Default|GetWB%20Inventaire%20Player%20UI%20Ref) "Visible")
      (Widget|SetVisibility (Variables|Default|GetWB%20Pause%20UI%20ref) "Hidden"))
    (:NewEnumerator8
      (Widget|SetVisibility (Variables|Default|GetWB%20Inventaire%20Vente%20Marchand%20UI%20Ref) "Visible")
      (Widget|SetVisibility (Variables|Default|GetWB%20Pause%20UI%20ref) "Hidden"))
    (:NewEnumerator9
      (Widget|SetVisibility (Variables|Default|GetWB%20Inventaire%20Achat%20Marchand%20UI%20Ref) "Visible")
      (Widget|SetVisibility (Variables|Default|GetWB%20Pause%20UI%20ref) "Hidden"))))

(event EventBeginPlay
  (bind _returnvalue (UserInterface|CreateWidget "/Game/InterfaceUtilisateur/Widget/WB_MenuUI.WB_MenuUI_C"))
  (bind _output_get (Variables|Default|SetWB%20Menu%20UI%20Ref _returnvalue))
  (Widget|SetVisibility _output_get "Visible")
  (UserInterface|Viewport|AddtoViewport _output_get 0)
  (bind _returnvalue_2 (UserInterface|CreateWidget "/Game/InterfaceUtilisateur/Widget/WB_PauseUI.WB_PauseUI_C"))
  (bind _output_get_2 (Variables|Default|SetWB%20Pause%20UI%20ref _returnvalue_2))
  (Widget|SetVisibility _output_get_2 "Hidden")
  (UserInterface|Viewport|AddtoViewport _output_get_2 0)
  (bind _returnvalue_3 (UserInterface|CreateWidget "/Game/InterfaceUtilisateur/Widget/WB_SettingsUI.WB_SettingsUI_C"))
  (bind _output_get_3 (Variables|Default|SetWB%20Settings%20UI%20Ref _returnvalue_3))
  (Widget|SetVisibility _output_get_3 "Hidden")
  (UserInterface|Viewport|AddtoViewport _output_get_3 0)
  (bind _returnvalue_4 (UserInterface|CreateWidget "/Game/InterfaceUtilisateur/Widget/WB_ControlsUI.WB_ControlsUI_C"))
  (bind _output_get_4 (Variables|Default|SetWB%20Controls%20UI%20Ref _returnvalue_4))
  (Widget|SetVisibility _output_get_4 "Hidden")
  (UserInterface|Viewport|AddtoViewport _output_get_4 0)
  (bind _returnvalue_5 (UserInterface|CreateWidget "/Game/InterfaceUtilisateur/Widget/WB_AudioUI.WB_AudioUI_C"))
  (bind _output_get_5 (Variables|Default|SetWB%20Audio%20UI%20Ref _returnvalue_5))
  (Widget|SetVisibility _output_get_5 "Hidden")
  (UserInterface|Viewport|AddtoViewport _output_get_5 0)
  (bind _returnvalue_6 (UserInterface|CreateWidget "/Game/InterfaceUtilisateur/Widget/WB_GameUI.WB_GameUI_C"))
  (bind _output_get_6 (Variables|Default|SetWB%20Game%20UI%20Ref _returnvalue_6))
  (Widget|SetVisibility _output_get_6 "Hidden")
  (UserInterface|Viewport|AddtoViewport _output_get_6 0)
  (bind _returnvalue_7 (UserInterface|CreateWidget "/Game/InterfaceUtilisateur/Widget/WB_SelectionMarchandUI.WB_SelectionMarchandUI_C"))
  (bind _output_get_7 (Variables|Default|SetWB%20Selection%20Marchand%20UI%20Ref _returnvalue_7))
  (Widget|SetVisibility _output_get_7 "Hidden")
  (UserInterface|Viewport|AddtoViewport _output_get_7 0)
  (bind _returnvalue_8 (UserInterface|CreateWidget "/Game/InterfaceUtilisateur/Widget/WB_InventaireVenteMarchandUI.WB_InventaireVenteMarchandUI_C"))
  (bind _output_get_8 (Variables|Default|SetWB%20Inventaire%20Vente%20Marchand%20UI%20Ref _returnvalue_8))
  (Widget|SetVisibility _output_get_8 "Hidden")
  (UserInterface|Viewport|AddtoViewport _output_get_8 0)
  (bind _returnvalue_9 (UserInterface|CreateWidget "/Game/InterfaceUtilisateur/Widget/WB_InventaireAchatMarchandUI.WB_InventaireAchatMarchandUI_C"))
  (bind _output_get_9 (Variables|Default|SetWB%20Inventaire%20Achat%20Marchand%20UI%20Ref _returnvalue_9))
  (Widget|SetVisibility _output_get_9 "Hidden")
  (UserInterface|Viewport|AddtoViewport _output_get_9 0)
  (bind _returnvalue_10 (UserInterface|CreateWidget "/Game/InterfaceUtilisateur/Widget/WB_InventairePlayerUI.WB_InventairePlayerUI_C"))
  (bind _output_get_10 (Variables|Default|SetWB%20Inventaire%20Player%20UI%20Ref _returnvalue_10))
  (Widget|SetVisibility _output_get_10 "Hidden")
  (UserInterface|Viewport|AddtoViewport _output_get_10 0))

(event EventTick
  (params (DeltaSeconds :type Float%20%28single-precision%29)))

(fn ConstructionScript)