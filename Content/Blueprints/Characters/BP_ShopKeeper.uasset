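; BP_ShopKeeper is a shopkeeper NPC that opens a shop screen when the player walks into its ShopTrigger.
; On overlap it blends the player's view to itself, then after a short delay creates WB_ShopkeeperUI, passing itself as the NPC reference.
; It then switches to UI-only input with a visible cursor and hides the player character; nothing here reverses these changes.
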(event OnComponentBeginOverlap(ShopTrigger)
  (params (OverlappedComponent :type Primitive%20Component%20Object%20Reference) (OtherActor :type Actor%20Object%20Reference) (OtherComp :type Primitive%20Component%20Object%20Reference) (OtherBodyIndex :type Integer) (bFromSweep :type Boolean) (SweepResult :type Hit%20Result%20Structure%20%28by%20ref%29))
  (bind _returnvalue (Game|GetPlayerController 0))
  (if (== OtherActor (Game|GetPlayerCharacter 0))
    (Game|Player|SetViewTargetwithBlend (Game|GetPlayerController 0) self 1.0 "VTBlend_Linear" 0.0 false)
    (Utilities|FlowControl|Delay 1.2)
    (bind _returnvalue_2 (UserInterface|CreateWidget "/Game/InterfaceUtilisateur/Widget/WB_ShopkeeperUI.WB_ShopkeeperUI_C" 0 self))
    (UserInterface|Viewport|AddtoViewport _returnvalue_2 0)
    (Input|SetInputModeUIOnly _returnvalue 0 "DoNotLock")
    (Variables|/Script/Engine.PlayerController|SetbShowMouseCursor _returnvalue true)
    (Rendering|SetActorHiddenInGame (Game|GetPlayerCharacter 0) true)))

(fn ConstructionScript)