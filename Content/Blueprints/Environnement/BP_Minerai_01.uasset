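; BP_Minerai_01 is a mineable crystal ore node that reappears after being broken.
; A sphere overlap toggles whether it can be taken, without filtering which actor overlaps.
; GetHit reduces Life by the player's pickaxe level when one is in hand, then hides the mesh at zero and flags it empty.
; Respawn restores it after a random 30–60 second delay, rerolling Quantity, which this graph never grants to the player.
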(event OnComponentBeginOverlap(Sphere_ReachDestroy)
  (params (OverlappedComponent :type Primitive%20Component%20Object%20Reference) (OtherActor :type Actor%20Object%20Reference) (OtherComp :type Primitive%20Component%20Object%20Reference) (OtherBodyIndex :type Integer) (bFromSweep :type Boolean) (SweepResult :type Hit%20Result%20Structure%20%28by%20ref%29))
  (bind _output_get (Variables|Default|SetCanBeTook? true))
  (Development|PrintString (Utilities|String|ToString(Boolean) _output_get)))

(event OnComponentEndOverlap(Sphere_ReachDestroy)
  (params (OverlappedComponent :type Primitive%20Component%20Object%20Reference) (OtherActor :type Actor%20Object%20Reference) (OtherComp :type Primitive%20Component%20Object%20Reference) (OtherBodyIndex :type Integer))
  (bind _output_get (Variables|Default|SetCanBeTook? false))
  (Development|PrintString (Utilities|String|ToString(Boolean) _output_get)))

(event Custom|Respawn
  (Utilities|FlowControl|Delay (Math|Float|Lerp 3e+01 6e+01 (Math|Random|RandomFloat)))
  (Rendering|SetVisibility (Variables|Default|GetSM_CristauxTest_01) true false)
  (Variables|Default|SetVide? false)
  (Variables|Default|SetQuantity (Math|Random|RandomInteger 4))
  (Variables|Default|SetLife 1))

(event Custom|GetHit
  (if (not (Variables|Default|GetVide?))
    (if (Variables|Default|GetCanBeTook?)
      (if (Variables|/Game/Blueprints/Characters/BP_Player.BP_Player_C|GetPiocheInHand? (Variables|Default|GetBP%20Player%20Ref))
        (Variables|Default|SetLife (- (Variables|Default|GetLife) (Variables|/Game/Blueprints/Characters/BP_Player.BP_Player_C|GetPiocheLevel (Variables|Default|GetBP%20Player%20Ref))))
        (if (<= (Variables|Default|GetLife) 0)
          (Development|PrintString "JeTePioche")
          (Rendering|SetVisibility (Variables|Default|GetSM_CristauxTest_01) false false)
          (Variables|Default|SetVide? true)
          (CallFunction|Respawn))))))

(event EventBeginPlay
  (Variables|Default|SetLevel 1)
  (Variables|Default|SetQuantity (Math|Random|RandomInteger 4))
  (Variables|Default|SetLife 1)
  (bind _returnvalue (Actor|GetActorOfClass "/Game/Blueprints/Characters/BP_Player.BP_Player_C"))
  (Variables|Default|SetBP%20Player%20Ref _returnvalue))

(event Collision|EventActorBeginOverlap
  (params (OtherActor :type Actor%20Object%20Reference)))

(event EventTick
  (params (DeltaSeconds :type Float%20%28single-precision%29)))

(fn ConstructionScript)