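; BP_SpawnMinerai_01 is an environment spawn point that places a BP_Minerai_01 ore actor at its own transform on BeginPlay.
; Its Respawn event, not called within this Blueprint, waits a random 30 to 60 seconds between debug prints, then spawns a new ore.
; Clicking the static mesh sets the Vide (empty) flag, which Respawn neither reads nor resets.
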(event OnClicked(StaticMesh)
  (params (TouchedComponent :type Primitive%20Component%20Object%20Reference) (ButtonPressed :type Key%20Structure :default "None"))
  (if (not (Variables|Default|GetVide?))
    (Variables|Default|SetVide? true)))

(event Custom|Respawn
  (Development|PrintString "BientotRetour")
  (Utilities|FlowControl|Delay (Math|Float|Lerp 3e+01 6e+01 (Math|Random|RandomFloat)))
  (Development|PrintString "Retour")
  (Game|SpawnActorfromClass "/Game/Blueprints/Environnement/BP_Minerai_01.BP_Minerai_01_C" (Transformation|GetActorTransform) "Undefined" 0 0))

(event EventBeginPlay
  (Game|SpawnActorfromClass "/Game/Blueprints/Environnement/BP_Minerai_01.BP_Minerai_01_C" (Transformation|GetActorTransform) "Undefined" 0 0)
  (Variables|Default|SetVide? false))

(event Collision|EventActorBeginOverlap
  (params (OtherActor :type Actor%20Object%20Reference)))

(event EventTick
  (params (DeltaSeconds :type Float%20%28single-precision%29)))

(fn ConstructionScript)