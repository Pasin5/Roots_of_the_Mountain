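; Mineable ruby crystal that gives the player a random small quantity of rubies when hit, then respawns after a random delay.
; GetHit requires the player inside the destroy sphere, a high enough pickaxe level and bag space, otherwise asking the game mode for upgrade messages where relevant.
; Harvesting hides the mesh and disables collision until respawn.
; A detection sphere drives a Tick-based emissive ramp, brightening the crystal while the player is near.
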(event OnComponentBeginOverlap(Sphere_ReachDetection)
  (params (OverlappedComponent :type Primitive%20Component%20Object%20Reference) (OtherActor :type Actor%20Object%20Reference) (OtherComp :type Primitive%20Component%20Object%20Reference) (OtherBodyIndex :type Integer) (bFromSweep :type Boolean) (SweepResult :type Hit%20Result%20Structure%20%28by%20ref%29))
  ;[0.4999 1 0.9901] Detection
  (Utilities|Casting|CastToBP_Player OtherActor)
  (Variables|Default|SetDetected? true))

(event OnComponentEndOverlap(Sphere_ReachDetection)
  (params (OverlappedComponent :type Primitive%20Component%20Object%20Reference) (OtherActor :type Actor%20Object%20Reference) (OtherComp :type Primitive%20Component%20Object%20Reference) (OtherBodyIndex :type Integer))
  ;[0.4999 1 0.9901] Detection
  (Utilities|Casting|CastToBP_Player OtherActor)
  (Variables|Default|SetDetected? false))

(event OnComponentBeginOverlap(Sphere_ReachDestroy)
  (params (OverlappedComponent :type Primitive%20Component%20Object%20Reference) (OtherActor :type Actor%20Object%20Reference) (OtherComp :type Primitive%20Component%20Object%20Reference) (OtherBodyIndex :type Integer) (bFromSweep :type Boolean) (SweepResult :type Hit%20Result%20Structure%20%28by%20ref%29))
  ;[0.6391 0.5841 1] In Range
  (Utilities|Casting|CastToBP_Player OtherActor)
  (Variables|Default|SetCanBeTook? true))

(event OnComponentEndOverlap(Sphere_ReachDestroy)
  (params (OverlappedComponent :type Primitive%20Component%20Object%20Reference) (OtherActor :type Actor%20Object%20Reference) (OtherComp :type Primitive%20Component%20Object%20Reference) (OtherBodyIndex :type Integer))
  ;[0.6391 0.5841 1] In Range
  (Utilities|Casting|CastToBP_Player OtherActor)
  (Variables|Default|SetCanBeTook? false))

(event Custom|Respawn
  ;[0.6712 1 0.5849] Respawn
  (Utilities|FlowControl|Delay (Math|Float|Lerp 3e+01 6e+01 (Math|Random|RandomFloat)))
  (Rendering|SetVisibility (Variables|Default|GetSM_CristauxTest_01) true false)
  (Variables|Default|SetVide? false)
  (Variables|Default|SetQuantity (+ (Math|Random|RandomInteger 3) 1))
  (Variables|Default|SetLife 1)
  (Collision|SetCollisionEnabled (Variables|Default|GetSM_CristauxTest_01) "QueryAndPhysics")
  (Collision|SetCollisionEnabled (Variables|Default|GetSphere_ReachDetection) "QueryOnly")
  (Collision|SetCollisionEnabled (Variables|Default|GetSphere_ReachDestroy) "QueryOnly"))

(event Custom|GetHit
  (bind _bp_player_ref (Variables|Default|GetBP%20Player%20Ref))
  (bind _bp_player_ref_2 (Variables|Default|GetBP%20Player%20Ref))
  (bind _bp_player_ref_3 (Variables|Default|GetBP%20Player%20Ref))
  (bind _qtrubymax (Variables|/Game/Blueprints/Characters/BP_Player.BP_Player_C|GetQTRubyMax _bp_player_ref_3))
  ;[1 0.4375 0.4375] Destruction
  (Components|Activation|Activate (Variables|Default|GetNiagara) false)
  (if (not (Variables|Default|GetVide?))
    (if (Variables|Default|GetCanBeTook?)
      (if (>= (Variables|/Game/Blueprints/Characters/BP_Player.BP_Player_C|GetPiocheLevel (Variables|Default|GetBP%20Player%20Ref)) 3)
        (if (< (Variables|/Game/Blueprints/Characters/BP_Player.BP_Player_C|GetQTRuby _bp_player_ref_2) (Variables|/Game/Blueprints/Characters/BP_Player.BP_Player_C|GetQTRubyMax _bp_player_ref_2))
          (Rendering|SetVisibility (Variables|Default|GetSM_CristauxTest_01) false false)
          (Variables|Default|SetVide? true)
          (CallFunction|Respawn)
          (Variables|/Game/Blueprints/Characters/BP_Player.BP_Player_C|SetQTRuby _bp_player_ref (+ (Variables|/Game/Blueprints/Characters/BP_Player.BP_Player_C|GetQTRuby _bp_player_ref) (Variables|Default|GetQuantity)))
          (if (> (Variables|/Game/Blueprints/Characters/BP_Player.BP_Player_C|GetQTRuby _bp_player_ref_3) _qtrubymax)
            (Variables|/Game/Blueprints/Characters/BP_Player.BP_Player_C|SetQTRuby _bp_player_ref_3 _qtrubymax))
          (Collision|SetCollisionEnabled (Variables|Default|GetSM_CristauxTest_01) "NoCollision")
          (Collision|SetCollisionEnabled (Variables|Default|GetSphere_ReachDetection) "NoCollision")
          (Collision|SetCollisionEnabled (Variables|Default|GetSphere_ReachDestroy) "NoCollision")
          (else
            (Default|MsgNeedBetterBag (Variables|Default|GetBP%20Game%20Mode%20Base%2001%20Ref))))
        (else
          (Default|MsgNeedBetterPickaxe (Variables|Default|GetBP%20Game%20Mode%20Base%2001%20Ref)))))))

(event Custom|Glowing
  ;[1 0.9577 0.4914] Brightness
  (if (Variables|Default|GetVide?)
    (Rendering|Material|SetScalarParameterValueonMaterials (Variables|Default|GetSM_CristauxTest_01) "EmissiveColorMultiply" 1.0)
    (elif (Variables|Default|GetDetected?)
      (Rendering|Material|SetScalarParameterValueonMaterials (Variables|Default|GetSM_CristauxTest_01) "EmissiveColorMultiply" (Variables|Default|GetBrightness))
      (if (>= (Variables|Default|GetBrightness) 5.0)
        (Variables|Default|SetBrightness 5.0)
        (else
          (Variables|Default|SetBrightness (+ (Variables|Default|GetBrightness) 0.1))))
      (else
        (Rendering|Material|SetScalarParameterValueonMaterials (Variables|Default|GetSM_CristauxTest_01) "EmissiveColorMultiply" (Variables|Default|GetBrightness))
        (if (<= (Variables|Default|GetBrightness) 1.0)
          (Variables|Default|SetBrightness 1.0)
          (else
            (Variables|Default|SetBrightness (- (Variables|Default|GetBrightness) 0.2))))))))

(event EventBeginPlay
  (Variables|Default|SetLevel 3)
  (Variables|Default|SetQuantity (+ (Math|Random|RandomInteger 3) 1))
  (Variables|Default|SetLife 1)
  (bind _returnvalue (Actor|GetActorOfClass "/Game/Blueprints/Characters/BP_Player.BP_Player_C"))
  (Variables|Default|SetBP%20Player%20Ref _returnvalue)
  (bind _returnvalue_2 (Actor|GetActorOfClass "/Game/Blueprints/Characters/BP_GameModeBase_01.BP_GameModeBase_01_C"))
  (Variables|Default|SetBP%20Game%20Mode%20Base%2001%20Ref _returnvalue_2))

(event EventTick
  (params (DeltaSeconds :type Float%20%28single-precision%29))
  (CallFunction|Glowing))

(fn ConstructionScript)