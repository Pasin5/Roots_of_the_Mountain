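; Destructible wall actor that the player destroys by spending a bomb when entering its Sphere trigger.
; On overlap with a nonzero BombNumb, a DoOnce decrements the player's count, calls PlusMessageBomb on BP_GameModeBase_01 and destroys the wall.
; With no bombs, entering calls the GameMode's MessageBomb and leaving calls PlusMessageBomb.
; Player and GameMode references are cached on BeginPlay through GetActorOfClass.
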(event OnComponentBeginOverlap(Sphere)
  (params (OverlappedComponent :type Primitive%20Component%20Object%20Reference) (OtherActor :type Actor%20Object%20Reference) (OtherComp :type Primitive%20Component%20Object%20Reference) (OtherBodyIndex :type Integer) (bFromSweep :type Boolean) (SweepResult :type Hit%20Result%20Structure%20%28by%20ref%29))
  (bind _bp_player_ref (Variables|Default|GetBP%20Player%20Ref))
  (bind _asbp_player (Utilities|Casting|CastToBP_Player OtherActor))
  (if (!= (Variables|/Game/Blueprints/Characters/BP_Player.BP_Player_C|GetBombNumb _asbp_player) 0)
    (Utilities|FlowControl|DoOnce false
      (:Completed
        (Variables|/Game/Blueprints/Characters/BP_Player.BP_Player_C|SetBombNumb _bp_player_ref (- (Variables|/Game/Blueprints/Characters/BP_Player.BP_Player_C|GetBombNumb _bp_player_ref) 1))
        (Default|PlusMessageBomb (Variables|Default|GetBP%20Game%20Mode%20Base%2001%20Ref))
        (Actor|DestroyActor)))
    (else
      (Default|MessageBomb (Variables|Default|GetBP%20Game%20Mode%20Base%2001%20Ref)))))

(event OnComponentEndOverlap(Sphere)
  (params (OverlappedComponent :type Primitive%20Component%20Object%20Reference) (OtherActor :type Actor%20Object%20Reference) (OtherComp :type Primitive%20Component%20Object%20Reference) (OtherBodyIndex :type Integer))
  (bind _asbp_player (Utilities|Casting|CastToBP_Player OtherActor))
  (if (not (!= (Variables|/Game/Blueprints/Characters/BP_Player.BP_Player_C|GetBombNumb _asbp_player) 0))
    (Default|PlusMessageBomb (Variables|Default|GetBP%20Game%20Mode%20Base%2001%20Ref))))

(event EventBeginPlay
  (bind _returnvalue (Actor|GetActorOfClass "/Game/Blueprints/Characters/BP_Player.BP_Player_C"))
  (Variables|Default|SetBP%20Player%20Ref _returnvalue)
  (bind _returnvalue_2 (Actor|GetActorOfClass "/Game/Blueprints/Characters/BP_GameModeBase_01.BP_GameModeBase_01_C"))
  (Variables|Default|SetBP%20Game%20Mode%20Base%2001%20Ref _returnvalue_2))

(event Collision|EventActorBeginOverlap
  (params (OtherActor :type Actor%20Object%20Reference)))

(event EventTick
  (params (DeltaSeconds :type Float%20%28single-precision%29)))

(fn ConstructionScript)