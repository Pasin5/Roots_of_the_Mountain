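; Mineable iron (Fer) resource node that adds a random quantity of iron to BP_Player when hit.
; GetHit requires the player in reach with a pickaxe (Pioche) in hand; one below level two triggers a brief, spam-guarded WB_Message.
; A depleted node hides its crystal mesh, then respawns after a random delay.
; A detection sphere drives an emissive glow, ramped up or down each Tick.
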(event OnComponentBeginOverlap(Sphere_ReachDetection)
  (params (OverlappedComponent :type Primitive%20Component%20Object%20Reference) (OtherActor :type Actor%20Object%20Reference) (OtherComp :type Primitive%20Component%20Object%20Reference) (OtherBodyIndex :type Integer) (bFromSweep :type Boolean) (SweepResult :type Hit%20Result%20Structure%20%28by%20ref%29))
  ;[0.4999 1 0.9901] Detection
  (Utilities|Casting|CastToBP_Player OtherActor)
  (Variables|Default|SetDetected? true))

(event OnComponentEndOverlap(Sphere_ReachDetection)
  (params (OverlappedComponent :type Primitive%20Component%20Object%20Reference) (OtherActor :type Actor%20Object%20Reference) (OtherComp :type Primitive%20Component%20Object%20Reference) (OtherBodyIndex :type Integer))
  ;[0.4999 1 0.9901] Detection
  (Utilities|Casting|CastToBP_Player OtherActor)
  (Variables|Default|SetDetected? false))

(event OnComponentBeginOverlap(Sphere_ReachDestroy)
  (params (OverlappedComponent :type Primitive%20Component%20Object%20Reference) (OtherActor :type Actor%20Object%20Reference) (OtherComp :type Primitive%20Component%20Object%20Reference) (OtherBodyIndex :type Integer) (bFromSweep :type Boolean) (SweepResult :type Hit%20Result%20Structure%20%28by%20ref%29))
  ;[0.6391 0.5841 1] In Range
  (Utilities|Casting|CastToBP_Player OtherActor)
  (Variables|Default|SetCanBeTook? true))

(event OnComponentEndOverlap(Sphere_ReachDestroy)
  (params (OverlappedComponent :type Primitive%20Component%20Object%20Reference) (OtherActor :type Actor%20Object%20Reference) (OtherComp :type Primitive%20Component%20Object%20Reference) (OtherBodyIndex :type Integer))
  ;[0.6391 0.5841 1] In Range
  (Utilities|Casting|CastToBP_Player OtherActor)
  (Variables|Default|SetCanBeTook? false))

(event Custom|Respawn
  ;[0.6712 1 0.5849] Respawn
  (Utilities|FlowControl|Delay (Math|Float|Lerp 3e+01 6e+01 (Math|Random|RandomFloat)))
  (Rendering|SetVisibility (Variables|Default|GetSM_CristauxTest_01) true false)
  (Variables|Default|SetVide? false)
  (Variables|Default|SetQuantity (+ (Math|Random|RandomInteger 4) 1))
  (Variables|Default|SetLife 1))

(event Custom|GetHit
  (bind _bp_player_ref (Variables|Default|GetBP%20Player%20Ref))
  ;[1 0.4375 0.4375] Destruction
  (if (not (Variables|Default|GetVide?))
    (if (Variables|Default|GetCanBeTook?)
      (if (Variables|/Game/Blueprints/Characters/BP_Player.BP_Player_C|GetPiocheInHand? (Variables|Default|GetBP%20Player%20Ref))
        (if (>= (Variables|/Game/Blueprints/Characters/BP_Player.BP_Player_C|GetPiocheLevel (Variables|Default|GetBP%20Player%20Ref)) 2)
          (Variables|Default|SetLife (- (Variables|Default|GetLife) 1))
          (if (<= (Variables|Default|GetLife) 0)
            (Rendering|SetVisibility (Variables|Default|GetSM_CristauxTest_01) false false)
            (Variables|Default|SetVide? true)
            (CallFunction|Respawn)
            (Variables|/Game/Blueprints/Characters/BP_Player.BP_Player_C|SetQTFer _bp_player_ref (+ (Variables|/Game/Blueprints/Characters/BP_Player.BP_Player_C|GetQTFer _bp_player_ref) (Variables|Default|GetQuantity))))
          (elif (not (Variables|Default|GetNOSPam))
            (bind _returnvalue (UserInterface|CreateWidget "/Game/InterfaceUtilisateur/Widget/Messages/WB_Message.WB_Message_C"))
            (UserInterface|Viewport|AddtoViewport _returnvalue 0)
            (Variables|Default|SetNOSPam true)
            (Utilities|FlowControl|Delay 1.0)
            (Variables|Default|SetNOSPam false)
            (Widget|RemovefromParent _returnvalue)))))))

(event Custom|Glowing
  ;[1 0.9577 0.4914] Brightness
  (if (Variables|Default|GetVide?)
    (Rendering|Material|SetScalarParameterValueonMaterials (Variables|Default|GetSM_CristauxTest_01) "EmissiveColorMultiply" 1.0)
    (elif (Variables|Default|GetDetected?)
      (Rendering|Material|SetScalarParameterValueonMaterials (Variables|Default|GetSM_CristauxTest_01) "EmissiveColorMultiply" (Variables|Default|GetBrightness))
      (if (>= (Variables|Default|GetBrightness) 4.0)
        (Variables|Default|SetBrightness 4.0)
        (else
          (Variables|Default|SetBrightness (+ (Variables|Default|GetBrightness) 0.1))))
      (else
        (Rendering|Material|SetScalarParameterValueonMaterials (Variables|Default|GetSM_CristauxTest_01) "EmissiveColorMultiply" (Variables|Default|GetBrightness))
        (if (<= (Variables|Default|GetBrightness) 1.0)
          (Variables|Default|SetBrightness 1.0)
          (else
            (Variables|Default|SetBrightness (- (Variables|Default|GetBrightness) 0.2))))))))

(event EventBeginPlay
  ;[1 1 1] Start parameters
  (Variables|Default|SetLevel 2)
  (Variables|Default|SetQuantity (+ (Math|Random|RandomInteger 4) 1))
  (Variables|Default|SetLife 1)
  (bind _returnvalue (Actor|GetActorOfClass "/Game/Blueprints/Characters/BP_Player.BP_Player_C"))
  (Variables|Default|SetBP%20Player%20Ref _returnvalue))

(event Collision|EventActorBeginOverlap
  (params (OtherActor :type Actor%20Object%20Reference)))

(event EventTick
  (params (DeltaSeconds :type Float%20%28single-precision%29))
  (CallFunction|Glowing))

(fn ConstructionScript)