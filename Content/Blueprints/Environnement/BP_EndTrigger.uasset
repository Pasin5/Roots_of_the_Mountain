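; BP_EndTrigger is the level's end zone, which completes the game only when the player's pickaxe (PiocheLevel) is at level 4.
; On BeginPlay it caches the BP_Player and adds a hidden WB_Message widget to the viewport.
; A qualifying overlap by a Player-tagged actor shows WB_EndScreen, then reloads the current level after a short delay.
; Below that level, any overlap shows the message until the overlap ends.
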(event OnComponentBeginOverlap(EndTrigger)
  (params (OverlappedComponent :type Primitive%20Component%20Object%20Reference) (OtherActor :type Actor%20Object%20Reference) (OtherComp :type Primitive%20Component%20Object%20Reference) (OtherBodyIndex :type Integer) (bFromSweep :type Boolean) (SweepResult :type Hit%20Result%20Structure%20%28by%20ref%29))
  (if (== (Variables|/Game/Blueprints/Characters/BP_Player.BP_Player_C|GetPiocheLevel (Variables|Default|GetBP%20PLayer%20Ref)) 4)
    (if (Actor|ActorHasTag OtherActor "Player")
      (bind _returnvalue (UserInterface|CreateWidget "/Game/InterfaceUtilisateur/Widget/WB_EndScreen.WB_EndScreen_C"))
      (UserInterface|Viewport|AddtoViewport _returnvalue 0)
      (Utilities|FlowControl|Delay 3.0)
      (bind _returnvalue_2 (Game|GetCurrentLevelName true))
      (Game|OpenLevel(byName) (Utilities|String|StringToName _returnvalue_2)))
    (else
      (Widget|SetVisibility (Variables|Default|GetWB%20Message%20Ref) "Visible"))))

(event OnComponentEndOverlap(EndTrigger)
  (params (OverlappedComponent :type Primitive%20Component%20Object%20Reference) (OtherActor :type Actor%20Object%20Reference) (OtherComp :type Primitive%20Component%20Object%20Reference) (OtherBodyIndex :type Integer))
  (if (not (== (Variables|/Game/Blueprints/Characters/BP_Player.BP_Player_C|GetPiocheLevel (Variables|Default|GetBP%20PLayer%20Ref)) 4))
    (Widget|SetVisibility (Variables|Default|GetWB%20Message%20Ref) "Hidden")))

(event EventBeginPlay
  (bind _returnvalue (Actor|GetActorOfClass "/Game/Blueprints/Characters/BP_Player.BP_Player_C"))
  (Variables|Default|SetBP%20PLayer%20Ref _returnvalue)
  (bind _returnvalue_2 (UserInterface|CreateWidget "/Game/InterfaceUtilisateur/Widget/Messages/WB_Message.WB_Message_C"))
  (bind _output_get (Variables|Default|SetWB%20Message%20Ref _returnvalue_2))
  (UserInterface|Viewport|AddtoViewport _output_get 0)
  (Widget|SetVisibility _output_get "Hidden"))

(fn ConstructionScript)