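; BP_Item is an inventory item actor that can be picked up and removed from the world.
; On BeginPlay, an invalid ItemObject is filled from GetDefaultItemObject, which here just returns that same variable.
; PickUpItem prints a debug message, triggers DestroyItem and returns Item.
; DestroyItem waits briefly before destroying the actor.
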(event Custom|Destroy%20Item
  (Utilities|FlowControl|Delay 0.1)
  (Actor|DestroyActor))

(event EventBeginPlay
  (if (not (Utilities|IsValid (Variables|Default|GetItemObject)))
    (bind _itemobject (CallFunction|GetDefaultItemObject))
    (Variables|Default|SetItemObject _itemobject)))

(fn ConstructionScript)

(fn GetDefaultItemObject
  (return (Variables|Default|GetItemObject)))

(fn PickUpItem
  (Development|PrintString "Item Picked")
  (CallFunction|DestroyItem)
  (return (Variables|Default|GetItem)))