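; BP_DestructibleMur is a wall actor that a player can remove by walking into its Sphere trigger while holding a bomb.
; On overlap it checks HaveBomb on BP_Player, then either clears the flag and destroys itself or shows a WB_Message_2 widget.
; The flag is cleared through a player reference cached at BeginPlay.
; Leaving the sphere without a bomb removes the message.
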(event OnComponentBeginOverlap(Sphere)
  (params (OverlappedComponent :type Primitive%20Component%20Object%20Reference) (OtherActor :type Actor%20Object%20Reference) (OtherComp :type Primitive%20Component%20Object%20Reference) (OtherBodyIndex :type Integer) (bFromSweep :type Boolean) (SweepResult :type Hit%20Result%20Structure%20%28by%20ref%29))
  (bind _asbp_player (Utilities|Casting|CastToBP_Player OtherActor))
  (if (Variables|/Game/Blueprints/Characters/BP_Player.BP_Player_C|GetHaveBomb? _asbp_player)
    (Variables|/Game/Blueprints/Characters/BP_Player.BP_Player_C|SetHaveBomb? (Variables|Default|GetBP%20Player%20Ref) false)
    (Actor|DestroyActor)
    (else
      (bind _returnvalue (UserInterface|CreateWidget "/Game/InterfaceUtilisateur/Widget/WB_Message_2.WB_Message_2_C"))
      (UserInterface|Viewport|AddtoViewport _returnvalue 0))))

(event OnComponentEndOverlap(Sphere)
  (params (OverlappedComponent :type Primitive%20Component%20Object%20Reference) (OtherActor :type Actor%20Object%20Reference) (OtherComp :type Primitive%20Component%20Object%20Reference) (OtherBodyIndex :type Integer))
  (bind _asbp_player (Utilities|Casting|CastToBP_Player OtherActor))
  (if (not (Variables|/Game/Blueprints/Characters/BP_Player.BP_Player_C|GetHaveBomb? _asbp_player))
    (Widget|RemovefromParent (stale OnComponentBeginOverlap(Sphere) _returnvalue))))

(event EventBeginPlay
  (bind _returnvalue (Actor|GetActorOfClass "/Game/Blueprints/Characters/BP_Player.BP_Player_C"))
  (Variables|Default|SetBP%20Player%20Ref _returnvalue))

(event Collision|EventActorBeginOverlap
  (params (OtherActor :type Actor%20Object%20Reference)))

(event EventTick
  (params (DeltaSeconds :type Float%20%28single-precision%29)))

(fn ConstructionScript)